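; BP_StepWidget is a step in the step manager sequence that displays a logo widget for a timed period.
; BeginStep shows the referenced logo and starts a one-shot timer, with a separate event to hide the logo and start a second, shorter timer.
; StepFinished passes completion to the parent step class, and the construction script only calls its parent.
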(event Custom|HideWIdget
  (Default|HideWidget (Variables|Default|GetLogoRef))
  (Utilities|Time|SetTimerbyEvent (EventDispatchers|CreateEvent :!event StepFinished) 3.0))

(event EventBeginStep
  (params (StepManager :type BP%20Step%20Manager%20Object%20Reference))
  (|CallParentFunction StepManager)
  (Default|ShowWidget (Variables|Default|GetLogoRef))
  (Utilities|Time|SetTimerbyEvent (EventDispatchers|CreateEvent :!event Custom|HideWIdget) 5.0))

(event EventStepFinished
  (|CallParentFunction))

(fn ConstructionScript
  (|CallParentFunction))