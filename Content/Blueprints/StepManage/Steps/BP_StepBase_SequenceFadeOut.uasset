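; A step Blueprint for the step manager that plays a level sequence, named as a fade-out, and takes away player input.
; On BeginStep it runs the parent logic, plays the LevelSequence player and binds an event to its OnFinished.
; It then disables input on the first player's pawn, with no re-enable in this graph.
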(event EventBeginStep
  (params (StepManager :type BP%20Step%20Manager%20Object%20Reference))
  (bind _levelsequence (Variables|Default|GetLevelSequence))
  (bind _sequenceplayer (Variables|/Script/LevelSequence.LevelSequenceActor|GetSequencePlayer _levelsequence))
  (|CallParentFunction StepManager)
  (Sequencer|Player|Play _sequenceplayer :!class /Script/MovieScene.MovieSceneSequencePlayer)
  (EventDispatchers|BindEventtoOnFinished _sequenceplayer (EventDispatchers|CreateEvent :!event StepFinished))
  (Input|DisableInput (Game|Player|GetPlayerPawn 0) (Game|GetPlayerController 0)))

(fn ConstructionScript
  (|CallParentFunction))