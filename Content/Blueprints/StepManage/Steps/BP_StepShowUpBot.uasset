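; BP_StepShowUpBot is a step run by the StepManager that introduces the bot to the player.
; On begin it plays the appear montage on the bot's skeletal mesh, unhiding the actor after a short delay to mask the animation blend.
; When that montage completes, it shows a greeting on the player pawn's HUD and plays a wave montage.
; The step finishes when the wave completes.
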(event EventBeginStep
  (params (StepManager :type BP%20Step%20Manager%20Object%20Reference))
  (|CallParentFunction StepManager)
  (Animation|Montage|PlayMontage (Variables|/Game/Characters/NPC/RW1Bot/BP_Bot.BP_Bot_C|GetSK_RW1Bot (Variables|Default|GetBotRef)) "/Game/Characters/NPC/RW1Bot/Animations/AS_Appear_Montage.AS_Appear_Montage"
    (:then
      ;[1 1 1] HideBlendAnimation
      (Utilities|FlowControl|Delay 0.2)
      (Rendering|SetActorHiddenInGame (Variables|Default|GetBotRef) false))
    (:OnCompleted
      (Default|ShowText (Variables|/Game/Blueprints/Base/BP_RW1Pawn.BP_RW1Pawn_C|GetPlayerHUD (.AsBP%20RW1Pawn (Utilities|Casting|CastToBP_RW1Pawn (Game|Player|GetPlayerPawn 0)))) 3.0 "Hello buddy!")
      (Animation|Montage|PlayMontage (Variables|/Game/Characters/NPC/RW1Bot/BP_Bot.BP_Bot_C|GetSK_RW1Bot (Variables|Default|GetBotRef)) "/Game/Characters/NPC/RW1Bot/Animations/AS_Wave_Montage.AS_Wave_Montage"
        (:OnCompleted
          (CallFunction|StepFinished))))))

(fn ConstructionScript
  (|CallParentFunction))