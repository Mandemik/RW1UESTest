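; BP_StepShowDevice is a tutorial step in which the bot presents devices and the player is told how to grab and rotate them.
; On begin, it sends the bot to the second level through its AI controller and listens for arrival.
; ShowDevice activates every BP_SimpleDevice cached at BeginPlay, shows the HUD circle and instructions, and plays a pointing montage.
; When the montage completes, it unlocks the bot's look-at-player.
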(event Custom|ShowDevice
  (bind _bot (Variables|Default|GetBot))
  (EventDispatchers|UnbindEventfromInPosition (.AsCustom%20AIControler (Utilities|Casting|CastToCustomAIControler (AI|GetAIController (Variables|Default|GetBot)))) (delegate Custom|ShowDevice))
  (for _array_element (Variables|Default|GetDeviceList)
    (Default|ActivateDevice _array_element))
  (Widget|SetVisibility (Variables|/Game/Widget/PlayerHuD.PlayerHuD_C|GetCircle (Variables|/Game/Blueprints/Base/BP_RW1Pawn.BP_RW1Pawn_C|GetPlayerHUD (.AsBP%20RW1Pawn (Utilities|Casting|CastToBP_RW1Pawn (Game|Player|GetPlayerPawn 0))))) "Visible")
  (Default|ShowText (Variables|/Game/Blueprints/Base/BP_RW1Pawn.BP_RW1Pawn_C|GetPlayerHUD (.AsBP%20RW1Pawn (Utilities|Casting|CastToBP_RW1Pawn (Game|Player|GetPlayerPawn 0)))) 1e+01 "Aim at the device and when it highlights, click and hold the left mouse button. Once you do this, hold down the right mouse button to rotate the object.")
  (Animation|Montage|PlayMontage (Variables|/Game/Characters/NPC/RW1Bot/BP_Bot.BP_Bot_C|GetSK_RW1Bot _bot) "/Game/Characters/NPC/RW1Bot/Animations/AS_PointLeft_Montage.AS_PointLeft_Montage"
    (:OnCompleted
      (Default|UnlockLookatPlayer (.AsCustom%20AIControler (Utilities|Casting|CastToCustomAIControler (AI|GetAIController _bot)))))))

(event EventBeginStep
  (params (StepManager :type BP%20Step%20Manager%20Object%20Reference))
  (bind _bot (Variables|Default|GetBot))
  (bind _returnvalue (AI|GetAIController _bot))
  (bind _ascustom_aicontroler (Utilities|Casting|CastToCustomAIControler _returnvalue))
  (|CallParentFunction StepManager)
  (Default|MovetoSecoundlLevel _ascustom_aicontroler)
  (EventDispatchers|BindEventtoInPosition _ascustom_aicontroler (EventDispatchers|CreateEvent :!event Custom|ShowDevice)))

(event EventBeginPlay
  (bind _outactors (Actor|GetAllActorsOfClass "/Game/Blueprints/BP_SimpleDevice.BP_SimpleDevice_C"))
  (for _array_element _outactors
    (Utilities|Array|Add (Variables|Default|GetDeviceList) _array_element)))

(fn ConstructionScript
  (|CallParentFunction))