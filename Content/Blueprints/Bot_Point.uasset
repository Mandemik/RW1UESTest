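; Bot_Point is a trigger point that signals a bot's arrival and turns it to the point's facing.
; The first BP_Bot to overlap its Box passes a DoOnce, is stored as BotRef, and has InSecoundPosition called on its CustomAIControler.
; A timeline then blends the bot's current rotation toward the point's actor rotation each update, using its Lerp track as alpha.
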(event OnComponentBeginOverlap(Box)
  (params (OverlappedComponent :type Primitive%20Component%20Object%20Reference) (OtherActor :type Actor%20Object%20Reference) (OtherComp :type Primitive%20Component%20Object%20Reference) (OtherBodyIndex :type Integer) (bFromSweep :type Boolean) (SweepResult :type Hit%20Result%20Structure%20%28by%20ref%29))
  (bind _asbp_bot (Utilities|Casting|CastToBP_Bot OtherActor))
  (Utilities|FlowControl|DoOnce false
    (:Completed
      (Variables|Default|SetBotRef _asbp_bot)
      (Default|InSecoundPosition (.AsCustom%20AIControler (Utilities|Casting|CastToCustomAIControler (AI|GetAIController (Variables|Default|GetBotRef)))))
      (bind _lerp (Timeline|Timeline_0 Play)
        (:Update
          (Transformation|SetActorRotation (Variables|Default|GetBotRef) (Math|Rotator|Lerp(Rotator) (Transformation|GetActorRotation (Variables|Default|GetBotRef)) (Transformation|GetActorRotation) _lerp)))))))

(fn ConstructionScript)