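; BP_SimpleDevice is a device actor that travels between a pedestal and the player.
; It records its starting transform and stays hidden without collision until activated.
; MovetoPlayer plays a timeline lerping it to the passed component's location and scale while keeping its own rotation.
; BackToPiedestal attaches to the pedestal and lerps back to the start, with each move stopping the opposite timeline and starting from the current transform.
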(event Custom|BackToPiedestal
  (Variables|Default|SetLastTransfomr (Transformation|GetActorTransform))
  (Transformation|AttachComponentToComponent (Variables|/Script/Engine.Actor|GetRootComponent (Variables|Default|GetPiedestal)) "None" "KeepRelative" "KeepRelative" "KeepRelative" true)
  (Utilities|FlowControl|Sequence
    (:then_0
      (bind _alpha (Timeline|Timeline_1 Stop)
        (:Update
          (Transformation|SetActorTransform (Math|Transform|Lerp(Transform) (Variables|Default|GetLastTransfomr) (Math|Transform|MakeTransform (.location (Transformation|GetWorldTransform (stale Custom|Move%20to%20Player RootTransform))) (Transformation|GetActorRotation) (.scale (Transformation|GetWorldTransform (stale Custom|Move%20to%20Player RootTransform)))) _alpha)))))
    (:then_1
      (bind _alpha_2 (Timeline|Timeline_0 PlayFromStart)
        (:Update
          (Transformation|SetActorTransform (Math|Transform|Lerp(Transform) (Variables|Default|GetLastTransfomr) (Variables|Default|GetStartingTransform) _alpha_2)))))))

(event Custom|Move%20to%20Player
  (params (RootTransform :type Scene%20Component%20Object%20Reference%20%28by%20ref%29))
  (bind _returnvalue (Transformation|GetWorldTransform RootTransform))
  (Variables|Default|SetLastTransfomr (Transformation|GetActorTransform))
  (Utilities|FlowControl|Sequence
    (:then_0
      (bind _alpha (Timeline|Timeline_0 Stop)
        (:Update
          (Transformation|SetActorTransform (Math|Transform|Lerp(Transform) (Variables|Default|GetLastTransfomr) (Variables|Default|GetStartingTransform) _alpha)))))
    (:then_1
      (bind _alpha_2 (Timeline|Timeline_1 PlayFromStart)
        (:Update
          (Transformation|SetActorTransform (Math|Transform|Lerp(Transform) (Variables|Default|GetLastTransfomr) (Math|Transform|MakeTransform (.location _returnvalue) (Transformation|GetActorRotation) (.scale _returnvalue)) _alpha_2)))))))

(event Custom|ActivateDevice
  (bind _staticmesh (Variables|Default|GetStaticMesh))
  (Development|SetHiddeninGame _staticmesh false false)
  (Collision|SetCollisionEnabled _staticmesh "QueryAndPhysics"))

(event Custom|DeactiveDevice
  (bind _staticmesh (Variables|Default|GetStaticMesh))
  (Development|SetHiddeninGame _staticmesh true false)
  (Collision|SetCollisionEnabled _staticmesh "NoCollision"))

(event EventBeginPlay
  (Variables|Default|SetStartingTransform (Transformation|GetActorTransform))
  (CallFunction|DeactiveDevice))

(fn ConstructionScript)