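; BP_RW1Pawn is a player pawn for inspecting BP_SimpleDevice objects, with mouse look and movement input, although BeginPlay disables character movement and creates the HUD.
; Capsule overlaps outline nearby devices through custom depth stencil.
; Holding SelectItem pulls the first overlapping device to SceenRoot and hides the HUD circle; release returns it to its pedestal.
; While EnableRotating is held, look input rotates the held device instead of the camera.
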(event OnComponentBeginOverlap(Capsule)
  (params (OverlappedComponent :type Primitive%20Component%20Object%20Reference) (OtherActor :type Actor%20Object%20Reference) (OtherComp :type Primitive%20Component%20Object%20Reference) (OtherBodyIndex :type Integer) (bFromSweep :type Boolean) (SweepResult :type Hit%20Result%20Structure%20%28by%20ref%29))
  ;[1 1 1] Outline Logic
  (bind _asbp_simple_device (Utilities|Casting|CastToBP_SimpleDevice OtherActor))
  (Utilities|IsValid (Variables|Default|GetActorSelected)
    (:Is%20Not%20Valid
      (CallFunction|TurnOutline _asbp_simple_device true))))

(event OnComponentEndOverlap(Capsule)
  (params (OverlappedComponent :type Primitive%20Component%20Object%20Reference) (OtherActor :type Actor%20Object%20Reference) (OtherComp :type Primitive%20Component%20Object%20Reference) (OtherBodyIndex :type Integer))
  ;[1 1 1] Outline Logic
  (if (Actor|ActorHasTag OtherActor "Outline")
    (CallFunction|TurnOutline OtherActor false)))

(event EventBeginPlay
  ;[1 1 1] Init
  (Pawn|Components|CharacterMovement|DisableMovement (Variables|Character|GetCharacterMovement))
  (bind _returnvalue (UserInterface|CreateWidget "/Game/Widget/PlayerHuD.PlayerHuD_C" (Game|GetPlayerController 0)))
  (bind _output_get (Variables|Default|SetPlayerHUD _returnvalue))
  (UserInterface|Viewport|AddtoViewport _output_get 0))

(event Input|ActionEvents|InputActionSelectItem
  (params (Key :type Key%20Structure :default "None"))
  ;[1 1 1] Inputs
  (:Pressed
    (CallFunction|SelectActor))
  (:Released
    (CallFunction|DropActor)))

(event Input|ActionEvents|InputActionEnableRotating
  (params (Key :type Key%20Structure :default "None"))
  ;[1 1 1] Inputs
  (:Pressed
    (Variables|Default|SetRotatingObject true))
  (:Released
    (Variables|Default|SetRotatingObject false)))

(event Input|AxisEvents|InputAxisMoveForward
  (params (AxisValue :type Float%20%28single-precision%29))
  ;[1 1 1] Inputs
  (Pawn|Input|AddMovementInput (Transformation|GetActorForwardVector) AxisValue false))

(event Input|AxisEvents|InputAxisMoveRight
  (params (AxisValue :type Float%20%28single-precision%29))
  ;[1 1 1] Inputs
  (Pawn|Input|AddMovementInput (Transformation|GetActorRightVector) AxisValue false))

(event Input|AxisEvents|InputAxisLookUp
  (params (AxisValue :type Float%20%28single-precision%29))
  ;[1 1 1] Inputs
  (if (and (Variables|Default|GetRotatingObject) (Utilities|IsValid (Variables|Default|GetActorSelected)))
    (CallFunction|RostateActor 0.0 AxisValue)
    (else
      (Pawn|Input|AddControllerPitchInput (* AxisValue (Variables|Default|GetMouseSpeed))))))

(event Input|AxisEvents|InputAxisTurn
  (params (AxisValue :type Float%20%28single-precision%29))
  ;[1 1 1] Inputs
  (if (and (Variables|Default|GetRotatingObject) (Utilities|IsValid (Variables|Default|GetActorSelected)))
    (CallFunction|RostateActor AxisValue 0.0)
    (else
      (Pawn|Input|AddControllerYawInput (* AxisValue (Variables|Default|GetMouseSpeed))))))

(fn ConstructionScript)

(fn TurnOutline
  (params (Actor :type Actor%20Object%20Reference) (On/Off :type Boolean))
  (bind _returnvalue (Actor|GetComponentbyClass Actor "/Script/Engine.StaticMeshComponent"))
  (bind _returnvalue_2 (Actor|GetComponentbyClass Actor "/Script/Engine.StaticMeshComponent"))
  (if On/Off
    (Rendering|SetRenderCustomDepth _returnvalue true)
    (Rendering|SetCustomDepthStencilValue _returnvalue 2)
    (else
      (Rendering|SetRenderCustomDepth _returnvalue_2 false)
      (Rendering|SetCustomDepthStencilValue _returnvalue_2 0))))

(fn SelectActor
  (bind _sceenroot (Variables|Default|GetSceenRoot))
  (bind _capsule (Variables|Default|GetCapsule))
  (bind _overlappingactors (Collision|GetOverlappingActors _capsule "/Game/Blueprints/BP_SimpleDevice.BP_SimpleDevice_C" :!class /Script/Engine.PrimitiveComponent))
  (if (Utilities|Array|IsValidIndex _overlappingactors)
    (Variables|Default|SetActorSelected (.AsBP%20Simple%20Device (Utilities|Casting|CastToBP_SimpleDevice (Utilities|Array|Get(acopy) _overlappingactors))))
    (Default|MovetoPlayer (Variables|Default|GetActorSelected) _sceenroot)
    (CallFunction|TurnOutline (Variables|Default|GetActorSelected) false)
    (Transformation|AttachComponentToComponent (Variables|Default|GetActorSelected) _sceenroot "None" "KeepRelative" "KeepRelative" "KeepRelative" true)
    (Widget|SetVisibility (Variables|/Game/Widget/PlayerHuD.PlayerHuD_C|GetCircle (Variables|Default|GetPlayerHUD)) "Collapsed")))

(fn DropActor
  (Utilities|IsValid (Variables|Default|GetActorSelected)
    (:Is%20Valid
      (Default|BacktoPiedestal (Variables|Default|GetActorSelected))
      (CallFunction|TurnOutline (Variables|Default|GetActorSelected) true)
      (Variables|Default|SetActorSelected 0)
      (Widget|SetVisibility (Variables|/Game/Widget/PlayerHuD.PlayerHuD_C|GetCircle (Variables|Default|GetPlayerHUD)) "Visible"))))

(fn RostateActor
  (params (TurnAxis :type Float%20%28single-precision%29) (LookUpAxis :type Float%20%28single-precision%29))
  (bind _actorselected (Variables|Default|GetActorSelected))
  (bind _returnvalue (Transformation|GetActorRotation _actorselected))
  (Transformation|SetActorRotation (Variables|Default|GetActorSelected) (Math|Rotator|MakeRotator (.roll _returnvalue) (+ (.pitch _returnvalue) LookUpAxis) (+ TurnAxis (.yaw _returnvalue)))))