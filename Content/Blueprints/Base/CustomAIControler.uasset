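; AI controller for BP_Bot that runs the BT_Bot behavior tree and drives it through blackboard keys.
; On BeginPlay it stores the player pawn, the bot's second location and a look-at-player flag.
; Events switch the bot between watching the player and moving to the second position, and arrival there clears the move flag and calls CallInPosition.
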(event Custom|MoveToSecoundlLevel
  (AI|Components|Blackboard|SetValueasBool (AI|GetBlackboard 0) (Utilities|Name|MakeLiteralName "MoveToSecound") true)
  (AI|Components|Blackboard|SetValueasBool (AI|GetBlackboard 0) (Utilities|Name|MakeLiteralName "LookAtPlayer") false))

(event Custom|InSecoundPosition
  (AI|Components|Blackboard|SetValueasBool (AI|GetBlackboard 0) (Utilities|Name|MakeLiteralName "MoveToSecound") false)
  (Default|CallInPosition))

(event Custom|UnlockLookAtPlayer
  (AI|Components|Blackboard|SetValueasBool (AI|GetBlackboard 0) (Utilities|Name|MakeLiteralName "LookAtPlayer") true))

(event EventBeginPlay
  ;[1 1 1] Init
  (AI|RunBehaviorTree "/Game/Blueprints/Base/BT_Bot.BT_Bot")
  (AI|Components|Blackboard|SetValueasObject (AI|GetBlackboard 0) (Utilities|Name|MakeLiteralName "PlayerKey") (Game|Player|GetPlayerPawn 0))
  (AI|Components|Blackboard|SetValueasVector (AI|GetBlackboard 0) (Utilities|Name|MakeLiteralName "SecoundPosition") (Transformation|GetActorLocation (Variables|/Game/Characters/NPC/RW1Bot/BP_Bot.BP_Bot_C|GetSecoundLocation (.AsBP%20Bot (Utilities|Casting|CastToBP_Bot (Pawn|GetControlledPawn))))))
  (AI|Components|Blackboard|SetValueasBool (AI|GetBlackboard 0) (Utilities|Name|MakeLiteralName "LookAtPlayer") true))

(fn ConstructionScript)