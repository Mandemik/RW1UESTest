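; BP_StepFadeIn is a Step Manager step that plays a referenced level sequence, presumably a fade-in.
; On BeginStep it calls the parent, disables input on the first player's pawn and starts the sequence player.
; It then binds an event to the sequence's OnFinished delegate; this graph does not re-enable input.
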(event EventBeginStep
  (params (StepManager :type BP%20Step%20Manager%20Object%20Reference))
  (bind _sequenceref (Variables|Default|GetSequenceRef))
  (bind _sequenceplayer (Variables|/Script/LevelSequence.LevelSequenceActor|GetSequencePlayer _sequenceref))
  (|CallParentFunction StepManager)
  (Input|DisableInput (Game|Player|GetPlayerPawn 0) (Game|GetPlayerController 0))
  (Sequencer|Player|Play _sequenceplayer :!class /Script/MovieScene.MovieSceneSequencePlayer)
  (EventDispatchers|BindEventtoOnFinished _sequenceplayer (EventDispatchers|CreateEvent :!event StepFinished)))

(fn ConstructionScript
  (|CallParentFunction))