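; BP_StepBotEnableMovement is a tutorial step, run by a StepManager, that unlocks player movement while the bot presents the controls.
; On BeginStep it enables the player pawn's input, sets its movement mode to walking and shows a timed HUD hint about moving and looking around.
; It also starts a one-shot timer matching the hint's duration and plays a talking montage on the bot's skeletal mesh.
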(event EventBeginStep
  (params (StepManager :type BP%20Step%20Manager%20Object%20Reference))
  (|CallParentFunction StepManager)
  (Input|EnableInput (Game|Player|GetPlayerPawn 0) (Game|GetPlayerController 0))
  (Pawn|Components|CharacterMovement|SetMovementMode (Variables|/Script/Engine.Character|GetCharacterMovement (.AsBP%20RW1Pawn (Utilities|Casting|CastToBP_RW1Pawn (Game|Player|GetPlayerPawn 0)))) "MOVE_Walking" 0)
  (Default|ShowText (Variables|/Game/Blueprints/Base/BP_RW1Pawn.BP_RW1Pawn_C|GetPlayerHUD (.AsBP%20RW1Pawn (Utilities|Casting|CastToBP_RW1Pawn (Game|Player|GetPlayerPawn 0)))) 8.0 "You can move by pressing WSAD,and look around with the mouse.  ")
  (Utilities|Time|SetTimerbyEvent (EventDispatchers|CreateEvent :!event StepFinished) 8.0)
  (Animation|Montage|PlayMontage (Variables|/Game/Characters/NPC/RW1Bot/BP_Bot.BP_Bot_C|GetSK_RW1Bot (Variables|Default|GetBotRef)) "/Game/Characters/NPC/RW1Bot/Animations/AS_TalkingPresentRight_Montage.AS_TalkingPresentRight_Montage"))

(fn ConstructionScript
  (|CallParentFunction))