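; BP_StepShowWidget is a step Blueprint for a step manager that displays a referenced 3D widget for a timed period.
; BeginStep calls the parent logic, shows the widget and starts a one-shot timer.
; A HideWidget event hides the widget and starts a second, shorter one-shot timer, whose bound event is not shown.
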(event Custom|HideWidget
  (Default|HideWidget (Variables|Default|GetWidget3DRef))
  (Utilities|Time|SetTimerbyEvent (EventDispatchers|CreateEvent :!event StepFinished) 2.0))

(event EventBeginStep
  (params (StepManager :type BP%20Step%20Manager%20Object%20Reference))
  (|CallParentFunction StepManager)
  (Default|ShowWidget (Variables|Default|GetWidget3DRef))
  (Utilities|Time|SetTimerbyEvent (EventDispatchers|CreateEvent :!event Custom|HideWidget) 8.0))

(fn ConstructionScript
  (|CallParentFunction))