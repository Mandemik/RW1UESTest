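; Tutorial step that introduces the player to selecting and rotating devices.
; BeginStep sends the bot to its second level through CustomAIControler and binds to that controller's in-position event.
; On arrival it unbinds, shows mouse-control instructions on the player HUD and plays the bot's point-left montage.
; All BP_SimpleDevice actors cached at BeginPlay activate as the montage starts; its completion unlocks the bot's look-at-player.
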(event Custom|BotInPosition
  (EventDispatchers|UnbindEventfromInPosition (.AsCustom%20AIControler (Utilities|Casting|CastToCustomAIControler (AI|GetAIController (Variables|Default|GetBotRef)))) (delegate Custom|BotInPosition))
  (Default|ShowText (Variables|/Game/Blueprints/Base/BP_RW1Pawn.BP_RW1Pawn_C|GetPlayerHUD (.AsBP%20RW1Pawn (Utilities|Casting|CastToBP_RW1Pawn (Game|Player|GetPlayerPawn 0)))) 8.0 "Aim at the device and when it highlights, click and hold the left mouse button. Onse you do this, hold down the right mouse button to rotate the object.")
  (Animation|Montage|PlayMontage (Variables|/Game/Characters/NPC/RW1Bot/BP_Bot.BP_Bot_C|GetSK_RW1Bot (Variables|Default|GetBotRef)) "/Game/Characters/NPC/RW1Bot/Animations/AS_PointLeft_Montage.AS_PointLeft_Montage"
    (:then
      (for _array_element (Variables|Default|GetDeviceList)
        (Default|ActivateDevice _array_element)))
    (:OnCompleted
      (Default|UnlockLookatPlayer (.AsCustom%20AIControler (Utilities|Casting|CastToCustomAIControler (AI|GetAIController (Variables|Default|GetBotRef))))))))

(event EventBeginPlay
  (bind _outactors (Actor|GetAllActorsOfClass "/Game/Blueprints/BP_SimpleDevice.BP_SimpleDevice_C"))
  (Variables|Default|SetDeviceList _outactors))

(event EventBeginStep
  (params (StepManager :type BP%20Step%20Manager%20Object%20Reference))
  (bind _botref (Variables|Default|GetBotRef))
  (bind _returnvalue (AI|GetAIController _botref))
  (bind _ascustom_aicontroler (Utilities|Casting|CastToCustomAIControler _returnvalue))
  (|CallParentFunction StepManager)
  (Default|MovetoSecoundlLevel _ascustom_aicontroler)
  (EventDispatchers|BindEventtoInPosition _ascustom_aicontroler (EventDispatchers|CreateEvent :!event Custom|BotInPosition)))

(fn ConstructionScript
  (|CallParentFunction))