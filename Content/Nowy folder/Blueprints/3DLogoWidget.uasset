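; 3DLogoWidget is a Blueprint that shows and hides a logo widget placed in the world, paired with a sparks particle effect.
; ShowWidget plays the LogoWidget's Fade animation forward, then activates the PSparks component after a short delay.
; HideWidget plays the same animation in reverse and deactivates the sparks immediately.
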(event Custom|ShowWidget
  (bind _aslogo_widget (Utilities|Casting|CastToLogoWidget (UserInterface|GetUserWidgetObject (Variables|Default|GetWidget))))
  (Class|UserWidget|PlayAnimationForward _aslogo_widget (Variables|/Game/Widget/LogoWidget.LogoWidget_C|GetFade _aslogo_widget) 1.0 false)
  (Utilities|FlowControl|Delay 1.0)
  (Components|Activation|SetActive (Variables|Default|GetP_Sparks) true false))

(event Custom|HideWidget
  (bind _aslogo_widget (Utilities|Casting|CastToLogoWidget (UserInterface|GetUserWidgetObject (Variables|Default|GetWidget))))
  (Class|UserWidget|PlayAnimationReverse _aslogo_widget (Variables|/Game/Widget/LogoWidget.LogoWidget_C|GetFade _aslogo_widget) 1.0 false)
  (Components|Activation|Deactivate (Variables|Default|GetP_Sparks)))

(fn ConstructionScript)